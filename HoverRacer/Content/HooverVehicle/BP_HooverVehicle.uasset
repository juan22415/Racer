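; BP_HooverVehicle is a physics-driven vehicle steered by angling its Motor component with the Turn axis.
; While Accelerate is held, Tick applies a steadily growing force to Cube at the Motor's location along its forward vector, resetting on release.
; Turn torque applies to Motor only when not accelerating.
; ForwardForce, set by Accelerate and the S key, is never read, so S has no effect on motion.
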(event EventTick
  (params (DeltaSeconds :type Float%20%28single-precision%29))
  (bind _motor (Variables|Default|Getmotor))
  (bind _motor_2 (Variables|Default|Getmotor))
  (if (Variables|Default|GetIsMoving)
    (bind _output_get (Variables|Default|SetActualForce (+ (Variables|Default|GetActualForce) (* (Utilities|Time|GetWorldDeltaSeconds) 6e+03))))
    (Class|PrimitiveComponent|AddForceatLocation (Variables|Default|GetCube) (* (Math|Vector|GetForwardVector _motor_2) _output_get) (Transformation|GetWorldLocation _motor_2) "None")
    (else
      (Class|PrimitiveComponent|AddTorqueinDegrees _motor (* (Math|Vector|GetUpVector _motor) (Variables|Default|GetTurnTorque)) "None" false)))
  (Transformation|SetRelativeRotation (Variables|Default|Getmotor) (Math|Rotator|MakeRotator 0.0 0.0 (* (Variables|Default|GetRotation%20Value) -3e+01)) false false))

(event Input|ActionEvents|InputActionAccelerate
  (params (Key :type Key%20Structure))
  (:Pressed
    (Variables|Default|SetForwardForce (Variables|Default|GetActualForce))
    (Variables|Default|SetIsMoving true))
  (:Released
    (Variables|Default|SetForwardForce 0.0)
    (Variables|Default|SetActualForce 5e+04)
    (Variables|Default|SetIsMoving false)))

(event Input|AxisEvents|InputAxisTurn
  (params (AxisValue :type Float%20%28single-precision%29))
  (bind _output_get (Variables|Default|SetRotation%20Value AxisValue))
  (Variables|Default|SetTurnTorque (* _output_get (Variables|Default|GettorqueForce))))

(event Input|KeyboardEvents|S
  (params (Key :type Key%20Structure))
  (:Pressed
    (Variables|Default|SetForwardForce -5e+04)))

(fn ConstructionScript)
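; Scene component that acts as a hover suspension point on a BP_HooverVehicle, pushing the vehicle away from the surface beneath it.
; Each tick it traces down its own up vector on the Visibility channel, up to the hover distance.
; On a hit, it applies a spring-damper force at its location to the vehicle's root primitive, using compression and its rate of change since the previous hit.
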(event EventBeginPlay
  (bind _asbp_hoover_vehicle (Utilities|Casting|CastToBP_HooverVehicle (Components|GetOwner)))
  (Variables|Default|SetParentVehicle _asbp_hoover_vehicle))

(event EventTick
  (params (DeltaSeconds :type Float%20%28single-precision%29))
  (bind _returnvalue (Transformation|GetWorldLocation))
  (Utilities|IsValid (Variables|Default|GetParentVehicle)
    (:Is%20Valid
      (bind (_outhit _returnvalue_2) (Collision|LineTraceByChannel _returnvalue (- _returnvalue (* (Math|Vector|GetUpVector) (Variables|Default|GetHooverDistance))) "TraceTypeQuery1" false 0 "None"))
      (if _returnvalue_2
        (bind _output_get (Variables|Default|SetHooverDelta (- (Variables|Default|GetHooverDistance) (.Distance (Collision|BreakHitResult _outhit)))))
        (Class|PrimitiveComponent|AddForceatLocation (.AsPrimitive%20Component (Utilities|Casting|CastToPrimitiveComponent (Variables|/Script/Engine.Actor|GetRootComponent (Variables|Default|GetParentVehicle)))) (* (Math|Vector|GetUpVector) (+ (* (/ (- _output_get (Variables|Default|GetPreviousHooverDelta)) (Utilities|Time|GetWorldDeltaSeconds)) (Variables|Default|GetDamping)) (* _output_get (Variables|Default|GetSpringCoefficient)))) (Transformation|GetWorldLocation) "None")
        (Variables|Default|SetPreviousHooverDelta (Variables|Default|GetHooverDelta))))))